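; BP_WaterPlane is a water plane actor that animates waves through its mesh's materials.
; On BeginPlay it starts the looping WaterWavesTimeline, whose scaled TimeLengthForWater track drives the "Time-Shift" scalar parameter on the static mesh materials.
; Tick is empty, and a disconnected alternative that accumulates a wrapping CurrentPhase from delta time remains in the graph but never runs.
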(event EventBeginPlay
  (Components|Timeline|SetLooping (Variables|Default|GetWater%20Waves%20Timeline) true)
  (bind _time_length_for_water (Timeline|Water%20Waves%20Timeline PlayFromStart)
    (:Update
      (Rendering|Material|SetScalarParameterValueonMaterials (Variables|Debug|GetStaticMeshComponent) "Time-Shift" (/ _time_length_for_water 5.0)))))

(event Collision|EventActorBeginOverlap
  (params (OtherActor :type Actor%20Object%20Reference)))

(event EventTick
  (params (DeltaSeconds :type Float%20%28single-precision%29)))

(fn ConstructionScript)
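; BP_PrintEnter is a state machine node used for testing that prints debug messages about its lifecycle.
; On Initialize it prints the node's display name with the given owner as world context, then calls the parent implementation.
; On Enter it looks up its state name from the owning machine and prints that the state is being entered.
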(event EventEnter
  (bind _returnvalue (Class|ProcStateMachine|GetStateName (Class|StateNode|GetMachine) self))
  (Development|PrintString (Class|StateNode|GetOwner) (Utilities|String|Append "Entering State: " (Utilities|String|ToString(Name) _returnvalue))))

(event EventInitialize
  (params (POwner :type Proc%20State%20Machine%20Object%20Reference))
  (Development|PrintString POwner (Utilities|String|Append "Initializing node: " (Utilities|GetDisplayName self)))
  (|CallParentFunction POwner))
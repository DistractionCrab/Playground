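; BP_LockOnCamera is a camera actor that turns to face a locked-on target.
; Its Sphere overlaps maintain a list of actors implementing BPI_Targetable, printing each one's name on entry.
; LockOn selects and returns the first listed actor, and Tick snaps the actor's rotation toward it while valid.
; LockOff clears the target and zeroes world rotation, and IsLockedOn reports whether a valid target exists.
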(event OnComponentBeginOverlap(Sphere)
  (params (OverlappedComponent :type Primitive%20Component%20Object%20Reference) (OtherActor :type Actor%20Object%20Reference) (OtherComp :type Primitive%20Component%20Object%20Reference) (OtherBodyIndex :type Integer) (bFromSweep :type Boolean) (SweepResult :type Hit%20Result%20Structure%20%28by%20ref%29))
  (Utilities|Casting|CastToBPI_Targetable OtherActor)
  (Development|PrintString (Utilities|GetDisplayName OtherActor))
  (Utilities|Array|Add (Variables|Default|GetPotential%20Targets) OtherActor))

(event OnComponentEndOverlap(Sphere)
  (params (OverlappedComponent :type Primitive%20Component%20Object%20Reference) (OtherActor :type Actor%20Object%20Reference) (OtherComp :type Primitive%20Component%20Object%20Reference) (OtherBodyIndex :type Integer))
  (Utilities|Array|RemoveItem (Variables|Default|GetPotential%20Targets) OtherActor))

(event EventBeginPlay)

(event Collision|EventActorBeginOverlap
  (params (OtherActor :type Actor%20Object%20Reference)))

(event EventTick
  (params (DeltaSeconds :type Float%20%28single-precision%29))
  (bind _lockontarget (Variables|Default|GetLockOnTarget))
  (if (Utilities|IsValid _lockontarget)
    (Transformation|SetActorRotation (Math|Rotator|FindLookatRotation (Transformation|GetActorLocation) (Transformation|GetActorLocation _lockontarget)))))

(fn ConstructionScript)

(fn Lockon
  (bind _potential_targets (Variables|Default|GetPotential%20Targets))
  (bind _potential_targets_2 (Variables|Default|GetPotential%20Targets))
  (bind _returnvalue (Utilities|Array|Length _potential_targets))
  (bind _output (Utilities|Array|Get(acopy) _potential_targets_2))
  (bind _returnvalue_2 (> _returnvalue 0))
  (bind _returnvalue_3 (select _returnvalue_2 _output 0))
  (Variables|Default|SetLockOnTarget _returnvalue_3)
  (return _returnvalue_3))

(fn IsLockedon
  (return (Utilities|IsValid (Variables|Default|GetLockOnTarget))))

(fn LockOff
  (Variables|Default|SetLockOnTarget 0)
  (Transformation|SetActorRotation "0, 0, 0"))
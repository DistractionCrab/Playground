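; BP_WaterOrb is a water orb spell actor that is channeled in the caster's hand and then launched.
; Initialize attaches it to the owner's right-hand socket, and channeling plays a timeline that scales the sphere.
; Launch detaches it, yaws its velocity toward the target or along the caster's facing, and enables tick movement plus sphere physics and gravity.
; The orb destroys itself when the sphere registers a hit.
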(event OnComponentHit(Sphere1)
  (params (HitComponent :type Primitive%20Component%20Object%20Reference) (OtherActor :type Actor%20Object%20Reference) (OtherComp :type Primitive%20Component%20Object%20Reference) (NormalImpulse :type Vector :default "0, 0, 0") (Hit :type Hit%20Result%20Structure%20%28by%20ref%29))
  (Actor|DestroyActor))

(event OnComponentBeginOverlap(Sphere1)
  (params (OverlappedComponent :type Primitive%20Component%20Object%20Reference) (OtherActor :type Actor%20Object%20Reference) (OtherComp :type Primitive%20Component%20Object%20Reference) (OtherBodyIndex :type Integer) (bFromSweep :type Boolean) (SweepResult :type Hit%20Result%20Structure%20%28by%20ref%29)))

(event EventBeginPlay)

(event EventTick
  (params (DeltaSeconds :type Float%20%28single-precision%29))
  (Transformation|AddActorWorldOffset (* DeltaSeconds (Variables|Default|GetVelocity))))

(event EventNotifyLaunch
  (params (Target :type Actor%20Object%20Reference))
  (bind _sphere1 (Variables|Default|GetSphere1))
  (CallFunction|LaunchOrb)
  (Physics|SetEnableGravity _sphere1 true)
  (Collision|SetCollisionEnabled _sphere1 "QueryAndPhysics")
  (Physics|SetSimulatePhysics _sphere1 true))

(event EventNotifyChannel
  (bind _scale (Timeline|Orb%20Channel%20Timeline PlayFromStart)
    (:Update
      (Transformation|SetRelativeTransform (Variables|Default|GetSphere1) (Math|Transform|MakeTransform "0, 0, 0" "0, 0, 0" (Math|Conversions|ToVector(Float) _scale)) false false))))

(fn ConstructionScript)

(fn LaunchOrb
  (Transformation|DetachFromActor "KeepWorld" "KeepWorld" "KeepRelative")
  (bind _get_self (Default|GetActor (Variables|Default|GetSpawning%20Actor)))
  (Actor|Tick|SetActorTickEnabled true)
  (if (Utilities|IsValid (Variables|Default|GetTarget))
    (Variables|Default|SetVelocity (Math|Vector|RotateVectorAroundAxis (Variables|Default|GetVelocity) (.yaw (Math|Rotator|FindLookatRotation (Transformation|GetActorLocation self) (Transformation|GetActorLocation (Variables|Default|GetTarget)))) "0.000000,0.000000,1.000000"))
    (else
      (Variables|Default|SetVelocity (Math|Vector|RotateVectorAroundAxis (Variables|Default|GetVelocity) (.yaw (Transformation|GetActorRotation _get_self)) "0.000000,0.000000,1.000000")))))

(fn Initialize
  (params (Owner%20Actor :type BPI%20Spell%20Caster%20Interface))
  (Default|AttachSpell Owner%20Actor "NewEnumerator0" "hand_rSocket" self)
  (Variables|Default|SetSpawning%20Actor Owner%20Actor))
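; BP_Spear is a melee weapon actor that damages RPG characters through separate head and body overlap components, with head hits dealing more damage.
; Activate and Deactivate toggle collision on both parts, and Deactivate also clears the list of hit actors.
; Overlaps feed HandleHit, which passes a constructed BP_HitOperator to each victim once per activation.
; Hitting a deflector interface actor instead starts deflection on the parent actor and deactivates the spear.
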(event OnComponentHit(Head)
  (params (HitComponent :type Primitive%20Component%20Object%20Reference) (OtherActor :type Actor%20Object%20Reference) (OtherComp :type Primitive%20Component%20Object%20Reference) (NormalImpulse :type Vector :default "0, 0, 0") (Hit :type Hit%20Result%20Structure%20%28by%20ref%29)))

(event OnComponentBeginOverlap(Head)
  (params (OverlappedComponent :type Primitive%20Component%20Object%20Reference) (OtherActor :type Actor%20Object%20Reference) (OtherComp :type Primitive%20Component%20Object%20Reference) (OtherBodyIndex :type Integer) (bFromSweep :type Boolean) (SweepResult :type Hit%20Result%20Structure%20%28by%20ref%29))
  (CallFunction|HandleHit OtherActor true))

(event OnComponentBeginOverlap(Body)
  (params (OverlappedComponent :type Primitive%20Component%20Object%20Reference) (OtherActor :type Actor%20Object%20Reference) (OtherComp :type Primitive%20Component%20Object%20Reference) (OtherBodyIndex :type Integer) (bFromSweep :type Boolean) (SweepResult :type Hit%20Result%20Structure%20%28by%20ref%29))
  (CallFunction|HandleHit OtherActor false))

(event EventBeginPlay)

(event Collision|EventActorBeginOverlap
  (params (OtherActor :type Actor%20Object%20Reference)))

(event EventTick
  (params (DeltaSeconds :type Float%20%28single-precision%29)))

(fn ConstructionScript)

(fn Activate
  (Collision|SetCollisionEnabled (Variables|Default|GetHead) "QueryAndPhysics")
  (Collision|SetCollisionEnabled (Variables|Default|GetBody) "QueryAndPhysics"))

(fn Deactivate
  (Collision|SetCollisionEnabled (Variables|Default|GetBody) "NoCollision")
  (Collision|SetCollisionEnabled (Variables|Default|GetHead) "NoCollision")
  (Utilities|Set|Clear (Variables|Default|GetHitActors)))

(fn HandleHit
  (params (Hit%20Actor :type Actor%20Object%20Reference) (Blade%20Hit? :type Boolean))
  (Utilities|Casting|CastToBPI_Deflector Hit%20Actor
    (:then
      (Class|PlaygroundCharacter|StartDeflection (Variables|Default|GetParentActor) true)
      (CallFunction|Deactivate))
    (:CastFailed
      (if (not (Utilities|Set|Contains (Variables|Default|GetHitActors)))
        (bind _asbpi_rpgcharacter (Utilities|Casting|CastToBPI_RPGCharacter Hit%20Actor))
        (bind _returnvalue (Game|ConstructObjectfromClass "/Game/Assets/Statistics/BP_HitOperator.BP_HitOperator_C" (select Blade%20Hit? 50 25)))
        (Default|ApplyDamage _asbpi_rpgcharacter _returnvalue)
        (Utilities|Set|Add (Variables|Default|GetHitActors) Hit%20Actor)))))
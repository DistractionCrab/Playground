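; BP_Lever is an interactable lever that rotates its handle and notifies activation listeners when the activation animation finishes.
; An overlap volume registers and unregisters the lever with BPI_Interactor actors.
; Timelines drive the handle's roll for activating, deactivating and matching a set activation state.
; CanInteract gates these animations and is toggled by Activate, Deactivate and the SetActivationState override.
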(event OnComponentBeginOverlap(InteractorCheck)
  (params (OverlappedComponent :type Primitive%20Component%20Object%20Reference) (OtherActor :type Actor%20Object%20Reference) (OtherComp :type Primitive%20Component%20Object%20Reference) (OtherBodyIndex :type Integer) (bFromSweep :type Boolean) (SweepResult :type Hit%20Result%20Structure%20%28by%20ref%29))
  (bind _asbpi_interactor (Utilities|Casting|CastToBPI_Interactor OtherActor))
  (Default|DeclareInteractable _asbpi_interactor self))

(event OnComponentEndOverlap(InteractorCheck)
  (params (OverlappedComponent :type Primitive%20Component%20Object%20Reference) (OtherActor :type Actor%20Object%20Reference) (OtherComp :type Primitive%20Component%20Object%20Reference) (OtherBodyIndex :type Integer))
  (bind _asbpi_interactor (Utilities|Casting|CastToBPI_Interactor OtherActor))
  (Default|RemoveInteractable _asbpi_interactor self))

(event Custom|ActivateEvent
  (if (Variables|Default|GetCanInteract)
    (bind _rotation_angle (Timeline|ActivateTimeline PlayFromStart)
      (:Update
        (CallFunction|UpdateHandleRotation _rotation_angle))
      (:Finished
        (Default|CallActivationListeners false self)))))

(event Custom|DeactivateEvent
  (if (Variables|Default|GetCanInteract)
    (bind _rotation_angle (Timeline|DeactivateTimeline PlayFromStart)
      (:Update
        (CallFunction|UpdateHandleRotation _rotation_angle)))))

(event Custom|SetHandleState
  (if (Variables|Default|GetCanInteract)
    (bind _rotation_angle (Timeline|HandleMotion ReverseFromEnd)
      (:Update
        (CallFunction|UpdateHandleRotation _rotation_angle)))
    (else
      (Timeline|HandleMotion PlayFromStart))))

(event EventInteract
  (params (Interactor :type Actor%20Object%20Reference))
  (CallFunction|ActivateEvent))

(fn ConstructionScript)

(fn Activate
  (CallFunction|ActivateEvent)
  (Variables|Default|SetCanInteract false))

(fn Deactivate
  (CallFunction|DeactivateEvent)
  (Variables|Default|SetCanInteract true))

(fn InteractInternal
  (if (Variables|Default|GetCanInteract)
    (CallFunction|Deactivate)
    (else
      (CallFunction|Activate))))

(fn UpdateHandleRotation
  (params (Handle%20Angle :type Float%20%28double-precision%29))
  (Transformation|SetRelativeRotation (Variables|Default|GetLeverHandle) (Math|Rotator|MakeRotator Handle%20Angle 0.0 0.0) false false))

(fn SetActivationState
  (params (ActivatedQ :type Boolean))
  (|CallParentFunction ActivatedQ)
  (Variables|Default|SetCanInteract (not ActivatedQ))
  (CallFunction|SetHandleState))

(fn DialogueText
  (return "Press E to Interact"))

(fn Transient
  (return true))
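; Elevator actor that travels one leg along an array of point actors each time its child pressure plate activates.
; A timeline curve scales the offset from the current point to the next to set actor location without sweep.
; On finish it raises the plate and steps the index, reversing at either end to ping-pong along the points.
; Start and end activators are bound, but their handlers are empty.
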(event Custom|StartActivate
  (params (ActivationQ :type Boolean)))

(event Custom|EndActivate
  (params (ActivationQ :type Boolean)))

(event Custom|PressurePlateActive
  (params (ActivateQ :type Boolean))
  (if (>= (Utilities|Array|Length (Variables|Default|GetPoints)) 2)
    (bind _elevation_curve (Timeline|Elevator%20Motion PlayFromStart)
      (:Update
        (Transformation|SetActorLocation (+ (* _elevation_curve (Utilities|MovementDirection)) (Utilities|MovementStart)) false false))
      (:Finished
        (Development|PrintString "waffles")
        (bind _asbp_pressure_plate (Utilities|Casting|CastToBP_PressurePlate (Variables|/Script/Engine.ChildActorComponent|GetChildActor (Variables|Default|GetPressurePlate))))
        (Default|PlateUp _asbp_pressure_plate)
        (CallFunction|UpdateStartIndex)))))

(event EventBeginPlay
  (EventDispatchers|BindEventtoActivationListeners (Variables|Default|GetStart%20Activator) (delegate Custom|StartActivate))
  (EventDispatchers|BindEventtoActivationListeners (Variables|Default|GetEnd%20Activator) (delegate Custom|EndActivate))
  (bind _asbp_abstract_activator (Utilities|Casting|CastToBP_AbstractActivator (Variables|/Script/Engine.ChildActorComponent|GetChildActor (Variables|Default|GetPressurePlate))))
  (EventDispatchers|BindEventtoActivationListeners _asbp_abstract_activator (delegate Custom|PressurePlateActive)))

(event Collision|EventActorBeginOverlap
  (params (OtherActor :type Actor%20Object%20Reference)))

(event EventTick
  (params (DeltaSeconds :type Float%20%28single-precision%29)))

(fn ConstructionScript)

(fn UpdateStartIndex
  (if (Variables|Default|GetReverse)
    ;[1 1 1] The case that the elevator is traveling in the reverse direction
    (if (>= (Utilities|Array|Length (Variables|Default|GetPoints)) 2)
      (bind _output_get (Variables|Default|SetPosition%20Index (+ (Variables|Default|GetPosition%20Index) -1)))
      (if (== _output_get 0)
        (Variables|Default|SetReverse false)))
    (else
      ;[1 1 1] The case that the elevator is traveling in the forward direction
      (if (>= (Utilities|Array|Length (Variables|Default|GetPoints)) 2)
        (bind _output_get_2 (Variables|Default|SetPosition%20Index (+ (Variables|Default|GetPosition%20Index) 1)))
        (if (== (+ _output_get_2 1) (Utilities|Array|Length (Variables|Default|GetPoints)))
          (Variables|Default|SetReverse true))))))
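; Elevator actor, apparently a backup, that moves between Points using a timeline elevation curve.
; A child-actor pressure plate starts the timeline, and finishing raises the plate, updates the position index and clears the two-index MovementSequence.
; PressurePlateActivate can fill that sequence but is not called here.
; Recall points bind only to debug prints, with the first activated at BeginPlay, and older ping-pong index logic is left disconnected.
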(event Custom|StartActivate
  (params (ActivationQ :type Boolean) (Source :type ABP%20Abstract%20Activator%20Object%20Reference))
  (Development|PrintString "activated"))

(event Custom|EndActivate
  (params (ActivationQ :type Boolean) (Source :type ABP%20Abstract%20Activator%20Object%20Reference))
  (Development|PrintString "endActivate"))

(event Custom|CustomEvent
  (if (>= (Utilities|Array|Length (Variables|Default|GetMovement%20Sequence)) 2)
    (bind _elevation_curve (Timeline|Elevator%20Motion%20Timeline PlayFromStart)
      (:Update
        (Transformation|SetActorLocation (+ (* _elevation_curve (Utilities|MovementDirection)) (Utilities|MovementStart)) false false))
      (:Finished
        (CallFunction|FinishMovement)))))

(event Custom|PressurePlateActive
  (params (ActivationQ :type Boolean) (Source :type ABP%20Abstract%20Activator%20Object%20Reference))
  (if (>= (Utilities|Array|Length (Variables|Default|GetPoints)) 2)
    (bind _elevation_curve (Timeline|Elevator%20Motion%20Timeline PlayFromStart)
      (:Update
        (Transformation|SetActorLocation (+ (* _elevation_curve (Utilities|MovementDirection)) (Utilities|MovementStart)) false false))
      (:Finished
        (CallFunction|FinishMovement)))))

(event EventBeginPlay
  (bind _recall_points (Variables|Default|GetRecall%20Points))
  (for _array_element _recall_points
    (EventDispatchers|BindEventtoActivationListeners _array_element (delegate Custom|StartActivate)))
  (for _array_element_2 _recall_points
    (EventDispatchers|BindEventtoActivationListeners _array_element_2 (delegate Custom|EndActivate)))
  (bind _asabp_abstract_activator (Utilities|Casting|CastToABP_AbstractActivator (Variables|/Script/Engine.ChildActorComponent|GetChildActor (Variables|Default|GetPressurePlate))))
  (EventDispatchers|BindEventtoActivationListeners _asabp_abstract_activator (delegate Custom|PressurePlateActive))
  (CallFunction|InitLevers))

(fn ConstructionScript)

(fn UpdateStartIndex
  (if (Utilities|TwoElementsQ)
    (Variables|Default|SetPosition%20Index (Utilities|Array|Get(acopy) (Variables|Default|GetMovement%20Sequence) 1))))

(fn InitLevers
  (if (> (Utilities|Array|Length (Variables|Default|GetRecall%20Points)) 0)
    (Default|SetActivationState (Utilities|Array|Get(acopy) (Variables|Default|GetRecall%20Points)) true)))

(fn FinishMovement
  (bind _asbp_pressure_plate (Utilities|Casting|CastToBP_PressurePlate (Variables|/Script/Engine.ChildActorComponent|GetChildActor (Variables|Default|GetPressurePlate))))
  (Default|PlateUp _asbp_pressure_plate)
  (CallFunction|UpdateStartIndex)
  (if (== (Utilities|Array|Length (Variables|Default|GetMovement%20Sequence)) 2)
    (Utilities|Array|Clear (Variables|Default|GetMovement%20Sequence))))

(fn UpdateElevatorLocation
  (params (Alpha :type Float%20%28double-precision%29))
  (Transformation|SetActorLocation (+ (* Alpha (Utilities|MovementDirection)) (Utilities|MovementStart)) false false))

(fn PressurePlateActivate
  (bind _points (Variables|Default|GetPoints))
  (bind _movement_sequence (Variables|Default|GetMovement%20Sequence))
  (bind _position_index (Variables|Default|GetPosition%20Index))
  (bind _returnvalue (Utilities|Array|Length _points))
  (bind _returnvalue_2 (+ _position_index 1))
  (if (>= _returnvalue 2)
    (Utilities|Array|Add _movement_sequence _position_index)
    (Utilities|Array|Add _movement_sequence (select (== _returnvalue_2 _returnvalue) (- _position_index 1) _returnvalue_2))))
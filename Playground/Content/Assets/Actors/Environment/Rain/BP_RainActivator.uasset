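; Rain trigger volume that starts or stops a BP_RainFollower when the PlaygroundCharacter enters, depending on ActivateQ.
; Activation reuses the tracked follower or spawns one, attached to the character with a raised relative offset.
; Deactivation only affects a tracked follower.
; RainActor is tracked through the follower's own overlaps with CollisionTrigger rather than stored on spawn, and cleared when that follower leaves.
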(event OnComponentBeginOverlap(CollisionTrigger)
  (params (OverlappedComponent :type Primitive%20Component%20Object%20Reference) (OtherActor :type Actor%20Object%20Reference) (OtherComp :type Primitive%20Component%20Object%20Reference) (OtherBodyIndex :type Integer) (bFromSweep :type Boolean) (SweepResult :type Hit%20Result%20Structure%20%28by%20ref%29))
  (CallFunction|HandleActivation OtherActor))

(event OnComponentEndOverlap(CollisionTrigger)
  (params (OverlappedComponent :type Primitive%20Component%20Object%20Reference) (OtherActor :type Actor%20Object%20Reference) (OtherComp :type Primitive%20Component%20Object%20Reference) (OtherBodyIndex :type Integer))
  (bind _asbp_rain_follower (Utilities|Casting|CastToBP_RainFollower OtherActor))
  (if (== (Variables|Default|GetRain%20Actor) _asbp_rain_follower)
    (Variables|Default|SetRain%20Actor 0)))

(event EventBeginPlay)

(event Collision|EventActorBeginOverlap
  (params (OtherActor :type Actor%20Object%20Reference)))

(event EventTick
  (params (DeltaSeconds :type Float%20%28single-precision%29)))

(fn ConstructionScript)

(fn HandleActivation
  (params (PGC%20or%20Rain :type Actor%20Object%20Reference))
  (bind _asplayground_character (Utilities|Casting|CastToPlaygroundCharacter PGC%20or%20Rain)
    (:then
      (if (Variables|Default|GetActivateQ)
        (if (Utilities|IsValid (Variables|Default|GetRain%20Actor))
          (Default|ActivateEvent (Variables|Default|GetRain%20Actor))
          (else
            (bind _returnvalue (Game|SpawnActorfromClass "/Game/Assets/Actors/Environment/Rain/BP_RainFollower.BP_RainFollower_C" (Math|Transform|MakeTransform "0.000000,0.000000,1000.000000") "Undefined" "MultiplyWithRoot" 0 0))
            (Transformation|AttachActorToActor _returnvalue _asplayground_character "None" "KeepRelative" "KeepWorld" "KeepWorld" true)
            (Default|ActivateEvent _returnvalue)))
        (elif (Utilities|IsValid (Variables|Default|GetRain%20Actor))
          (Default|DeactivateEvent (Variables|Default|GetRain%20Actor)))))
    (:CastFailed
      (bind _asbp_rain_follower (Utilities|Casting|CastToBP_RainFollower PGC%20or%20Rain))
      (Variables|Default|SetRain%20Actor _asbp_rain_follower))))
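; Rain actor that fades the density of its rain particle system in and out when activated or deactivated.
; ActivateEvent and DeactivateEvent run two opposing timelines that drive the RAINDENSITY variable, each stopping the other.
; Timeline start positions derive from the current-to-max density ratio, which only the fade-in updates.
; The fade-out uses a hardcoded peak density and destroys the actor when finished.
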(event Custom|Deactivate%20Event
  (Audio|Components|Audio|Stop (Variables|Default|GetIncrease%20Rain%20to%20Max))
  (bind _alpha_track (Timeline|Reduce%20Rain%20to%20Zero Play)
    (:Update
      (Niagara|SetNiagaraVariable(Float) (Variables|Default|GetRain%20System) "RAINDENSITY" (Math|Float|Lerp 0.0 3e+03 _alpha_track)))
    (:Finished
      (Actor|DestroyActor))))

(event Custom|Activate%20Event
  (Variables|Default|SetActivated true)
  (Audio|Components|Audio|Stop (Variables|Default|GetReduce%20Rain%20to%20zero))
  (bind _alpha (Timeline|Increase%20Rain%20to%20Max Play)
    (:Update
      (bind _output_get (Variables|ParticleVariables|SetCURRENT%20DENSITY (Math|Float|Lerp 0.0 (Variables|ParticleVariables|GetMAXDENSITY) _alpha)))
      (Niagara|SetNiagaraVariable(Float) (Variables|Default|GetRain%20System) "RAINDENSITY" _output_get))))

(event EventBeginPlay)

(event Collision|EventActorBeginOverlap
  (params (OtherActor :type Actor%20Object%20Reference)))

(event EventTick
  (params (DeltaSeconds :type Float%20%28single-precision%29)))

(fn ConstructionScript)
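; BP_Spellpickup is an interactable world item that grants the player a spell.
; On Interact, it casts the interactor to BP_PlaygroundCharacter and adds its SpellKey to that character's Inventory.
; It then builds a BP_TextOnlyDisplay showing the spell's icon and key, passes it to the character's DeclareInteractable, and destroys itself.
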(event EventBeginPlay
  (|CallParentFunction) ; This node is disabled and will not be called.\nDrag off pins to build functionality.
)

(event Collision|EventActorBeginOverlap
  (params (OtherActor :type Actor%20Object%20Reference))
  (|CallParentFunction OtherActor) ; This node is disabled and will not be called.\nDrag off pins to build functionality.
)

(event EventTick
  (params (DeltaSeconds :type Float%20%28single-precision%29))
  (|CallParentFunction DeltaSeconds) ; This node is disabled and will not be called.\nDrag off pins to build functionality.
)

(event EventInteract
  (params (Interactor :type Actor%20Object%20Reference))
  (bind _asbp_playground_character (Utilities|Casting|CastToBP_PlaygroundCharacter Interactor))
  (Default|AddSpell (Variables|/Game/Assets/Actors/Entity/Characters/MainCharacter/BP_PlaygroundCharacter.BP_PlaygroundCharacter_C|GetInventory _asbp_playground_character) (Variables|Default|GetSpellKey))
  (bind _returnvalue (Game|ConstructObjectfromClass "/Game/Assets/UI/BP_TextOnlyDisplay.BP_TextOnlyDisplay_C" (Utilities|Text|FormatText "<img id=\"{IconKey}\"/> {SpellKey}" (Variables|Default|GetIconKey) (Variables|Default|GetSpellKey))))
  (Default|DeclareInteractable _asbp_playground_character _returnvalue)
  (Actor|DestroyActor))

(fn ConstructionScript
  (|CallParentFunction))
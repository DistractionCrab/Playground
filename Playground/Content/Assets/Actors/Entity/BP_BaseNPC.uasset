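; BP_BaseNPC is a base NPC actor that exposes faction, health, response and patrol queries, with no event logic of its own.
; CanPatrol is true only when a valid PatrolPath has at least one patrol point.
; GetResponse looks up only the first element of the OtherEntity array in the Responses map, falling back to the first enum value when none is found.
; GetFactions and GetHealth are plain getters.
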(event EventBeginPlay)

(event Collision|EventActorBeginOverlap
  (params (OtherActor :type Actor%20Object%20Reference)))

(event EventTick
  (params (DeltaSeconds :type Float%20%28single-precision%29)))

(fn ConstructionScript)

(fn CanPatrol
  (if (Utilities|IsValid (Variables|Movement|GetPatrol%20Path))
    (return (> (Utilities|Array|Length (Variables|/Script/Playground.PatrolPath|GetPatrolPoints (Variables|Movement|GetPatrol%20Path))) 0))
    (else
      (return false))))

(fn GetFactions
  (return (Variables|RPGElements|GetFactions)))

(fn GetHealth
  (return (Variables|RPGElements|GetHealth)))

(fn GetResponse
  (params (Other%20Entity :type Array%20of%20BP_Factions%20Enums :default "NewEnumerator0"))
  (bind _output (Utilities|Array|Get(acopy) Other%20Entity))
  (bind _responses (Variables|RPGElements|GetResponses))
  (bind (_value _returnvalue) (Utilities|Map|Find _responses _output))
  (return (select (and _returnvalue (> (Utilities|Array|Length Other%20Entity) 0)) _value "NewEnumerator0")))
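; BP_WaterHuman is an entity actor for a water human that can take damage.
; Its ApplyDamage event prints a debug message and passes the incoming hit to Health through OperateValue.
; BeginPlay, overlap, Tick and the construction script add no logic of their own.
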(event EventBeginPlay
  (|CallParentFunction) ; This node is disabled and will not be called.\nDrag off pins to build functionality.
)

(event Collision|EventActorBeginOverlap
  (params (OtherActor :type Actor%20Object%20Reference))
  (|CallParentFunction OtherActor) ; This node is disabled and will not be called.\nDrag off pins to build functionality.
)

(event EventTick
  (params (DeltaSeconds :type Float%20%28single-precision%29))
  (|CallParentFunction DeltaSeconds) ; This node is disabled and will not be called.\nDrag off pins to build functionality.
)

(event EventApplyDamage
  (params (The%20Hit :type BP%20Hit%20Operator%20Object%20Reference))
  (Development|PrintString "Taking Damage")
  (Class|IntVariable|OperateValue (Variables|Default|GetHealth) The%20Hit))

(fn ConstructionScript
  (|CallParentFunction))
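; Test player character that turns directional keyboard input into movement axis values and hosts the main dialogue UI.
; On BeginPlay it adds the Enhanced Input mapping context, puts WBP_MainUI in the viewport and registers a state-change listener.
; That listener sets CharState on ABP_TestCharacter for Idle and Walking.
; DisplayPopup and HidePopup forward to the UI's dialogue, while UpdatePerspective is a stub returning a zero vector.
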(event Custom|Start%20Walking
  (params (From :type EMainCharacterState%20Enum :default "IDLE") (To :type EMainCharacterState%20Enum :default "IDLE"))
  (CallFunction|UpdateAnimState From To))

(event Input|EnhancedActionEvents|EnhancedInputActionIA_Forward
  (params (ActionValue :type Boolean) (ElapsedSeconds :type Float%20%28double-precision%29) (TriggeredSeconds :type Float%20%28double-precision%29) (InputAction :type Input%20Action%20Object%20Reference :default "/Game/Assets/Actors/Entity/Characters/Test/IA_Forward.IA_Forward"))
  (:Triggered
    (Class|MainCharacter|InputAxisX 1.0 :!label _label))
  (:Ongoing
    (goto _label))
  (:Canceled
    (Class|MainCharacter|InputAxisX 0.0 :!label _label_2))
  (:Completed
    (goto _label_2)))

(event Input|EnhancedActionEvents|EnhancedInputActionIA_Backward
  (params (ActionValue :type Boolean) (ElapsedSeconds :type Float%20%28double-precision%29) (TriggeredSeconds :type Float%20%28double-precision%29) (InputAction :type Input%20Action%20Object%20Reference :default "/Game/Assets/Actors/Entity/Characters/Test/IA_Backward.IA_Backward"))
  (:Triggered
    (Class|MainCharacter|InputAxisX -1.0 :!label _label))
  (:Ongoing
    (goto _label))
  (:Canceled
    (Class|MainCharacter|InputAxisX 0.0 :!label _label_2))
  (:Completed
    (goto _label_2)))

(event Input|EnhancedActionEvents|EnhancedInputActionIA_Left
  (params (ActionValue :type Boolean) (ElapsedSeconds :type Float%20%28double-precision%29) (TriggeredSeconds :type Float%20%28double-precision%29) (InputAction :type Input%20Action%20Object%20Reference :default "/Game/Assets/Actors/Entity/Characters/Test/IA_Left.IA_Left"))
  (:Triggered
    (Class|MainCharacter|InputAxisY -1.0 :!label _label))
  (:Ongoing
    (goto _label))
  (:Canceled
    (Class|MainCharacter|InputAxisY 0.0 :!label _label_2))
  (:Completed
    (goto _label_2)))

(event Input|EnhancedActionEvents|EnhancedInputActionIA_Right
  (params (ActionValue :type Boolean) (ElapsedSeconds :type Float%20%28double-precision%29) (TriggeredSeconds :type Float%20%28double-precision%29) (InputAction :type Input%20Action%20Object%20Reference :default "/Game/Assets/Actors/Entity/Characters/Test/IA_Right.IA_Right"))
  (:Triggered
    (Class|MainCharacter|InputAxisY 1.0 :!label _label))
  (:Ongoing
    (goto _label))
  (:Canceled
    (Class|MainCharacter|InputAxisY 0.0 :!label _label_2))
  (:Completed
    (goto _label_2)))

(event EventBeginPlay
  (CallFunction|InitInput)
  (CallFunction|InitInterface)
  (Class|MainCharacter|StateListen (delegate Custom|Start%20Walking)))

(event Collision|EventActorBeginOverlap
  (params (OtherActor :type Actor%20Object%20Reference)))

(event EventTick
  (params (DeltaSeconds :type Float%20%28single-precision%29)))

(fn ConstructionScript)

(fn DisplayPopup
  (params (DisplayText :type Text))
  (Default|DisplayDialogue (Variables|Default|GetMainUI) DisplayText))

(fn HidePopup
  (Default|HideDialogue (Variables|Default|GetMainUI)))

(fn InitInput
  (bind _asplayer_controller (Utilities|Casting|CastToPlayerController (Pawn|GetController)))
  (Input|AddMappingContext (PlayerController|LocalPlayerSubsystems|GetEnhancedInputLocalPlayerSubsystem _asplayer_controller) "/Game/Assets/Actors/Entity/Characters/Test/IMC_Keyboard.IMC_Keyboard" 0 "(bIgnoreAllPressedKeysUntilRelease=True,bForceImmediately=False)"))

(fn InitInterface
  (bind _asbp_main_ui (Utilities|Casting|CastToWBP_MainUI (UserInterface|GetWidget (Variables|Default|GetMain%20UI))))
  (bind _output_get (Variables|Default|SetMainUI _asbp_main_ui))
  (UserInterface|Viewport|AddtoViewport _output_get 0))

(fn UpdateAnimState
  (params (From :type EMainCharacterState%20Enum :default "IDLE") (To :type EMainCharacterState%20Enum :default "IDLE"))
  (bind _mesh (Variables|Character|GetMesh))
  (bind _returnvalue (Components|SkeletalMesh|GetAnimInstance _mesh))
  (switch Utilities|FlowControl|Switch|SwitchonEMainCharacterState To
    (:IDLE
      (bind _asabp_test_character (Utilities|Casting|CastToABP_TestCharacter _returnvalue))
      (Variables|/Game/Assets/Actors/Entity/Characters/Test/ABP_TestCharacter.ABP_TestCharacter_C|SetCharState _asabp_test_character "NewEnumerator1"))
    (:WALKING
      (bind _asabp_test_character_2 (Utilities|Casting|CastToABP_TestCharacter _returnvalue))
      (Variables|/Game/Assets/Actors/Entity/Characters/Test/ABP_TestCharacter.ABP_TestCharacter_C|SetCharState _asabp_test_character_2 "NewEnumerator0"))))

(fn UpdatePerspective
  (params (NewParam :type Vector))
  (return "0, 0, 0"))
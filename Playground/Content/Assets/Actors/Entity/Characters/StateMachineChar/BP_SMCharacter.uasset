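; BP_SMCharacter is a player character whose movement input drives a state machine, ProcStateMachine.
; On BeginPlay it adds the Enhanced Input mapping context and caches the WALKING state node.
; Move input sends walk and stop-walk events to the machine and feeds the axis to that node, while Look applies controller yaw and pitch directly.
; A movement-mode callback sends a "None" event when the character is falling.
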(event EventBeginPlay
  (Init|SetupInput)
  (Init|InitStateRefs))

(event Input|EnhancedActionEvents|EnhancedInputActionIA_Move
  (params (ActionValue :type Vector%202D%20Structure) (ElapsedSeconds :type Float%20%28double-precision%29) (TriggeredSeconds :type Float%20%28double-precision%29) (InputAction :type Input%20Action%20Object%20Reference :default "/Game/Assets/Input/IA_Move.IA_Move"))
  (:Triggered
    (Control|Movement|MovementContinue ActionValue))
  (:Started
    (Control|Movement|MovementStart))
  (:Canceled
    (Control|Movement|MovementStopped :!label _label))
  (:Completed
    (goto _label)))

(event Input|EnhancedActionEvents|EnhancedInputActionIA_Look
  (params (ActionValue :type Vector%202D%20Structure) (ElapsedSeconds :type Float%20%28double-precision%29) (TriggeredSeconds :type Float%20%28double-precision%29) (InputAction :type Input%20Action%20Object%20Reference :default "/Game/Assets/Input/IA_Look.IA_Look"))
  (:Triggered
    (Control|Camera|Look ActionValue)))

(fn ConstructionScript)

(fn InitStateRefs
  (bind _returnvalue (Class|ProcStateMachineComponent|FindNode (Variables|Default|GetProcStateMachine) "WALKING")
    (:FOUND
      (bind _asmovement_state_node (Utilities|Casting|CastToMovementStateNode _returnvalue))
      (Variables|StateMachine|States|SetWalkingStateNode _asmovement_state_node))))

(fn SetupInput
  (bind _asplayer_controller (Utilities|Casting|CastToPlayerController (Pawn|GetController)))
  (Input|AddMappingContext (PlayerController|LocalPlayerSubsystems|GetEnhancedInputLocalPlayerSubsystem _asplayer_controller) "/Game/Assets/Input/IMC_Default.IMC_Default" 0 "(bIgnoreAllPressedKeysUntilRelease=True,bForceImmediately=False)"))

(fn MovementStart
  (Class|ProcStateMachineComponent|Event (Variables|Default|GetProcStateMachine) (Variables|StateMachine|Events|Constants|GetWalkEventName)))

(fn MovementContinue
  (params (InputAxis :type Vector%202D%20Structure))
  (Class|MovementStateNode|UpdateInputAxis (Variables|StateMachine|States|GetWalkingStateNode) InputAxis)
  (Class|ProcStateMachineComponent|Event (Variables|Default|GetProcStateMachine) (Variables|StateMachine|Events|Constants|GetWalkEventName)))

(fn MovementStopped
  (Class|ProcStateMachineComponent|Event (Variables|Default|GetProcStateMachine) (Variables|StateMachine|Events|Constants|GetStopWalkEventName)))

(fn Look
  (params (LookAxis :type Vector%202D%20Structure))
  (Pawn|Input|AddControllerYawInput (.x LookAxis))
  (Pawn|Input|AddControllerPitchInput (.y LookAxis)))

(fn EVMovementModeChangedCallback
  (params (Component :type Event%20Char%20Movement%20Component%20Object%20Reference) (Previous :type EMovementMode%20Enum :default "MOVE_None") (PreviousCustom :type Byte))
  (if (AI|Components|NavMovement|IsFalling (Variables|Character|GetCharacterMovement))
    (Class|ProcStateMachineComponent|Event (Variables|Default|GetProcStateMachine) "None")))
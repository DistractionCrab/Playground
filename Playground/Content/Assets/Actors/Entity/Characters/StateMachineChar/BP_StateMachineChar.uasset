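; Character Blueprint that drives movement through a ProcStateMachine and sets up Enhanced Input on BeginPlay.
; Move input sends walk and stop-walk events to the state machine and feeds its axis into a cached WALKING MovementStateNode.
; Look input bypasses the state machine to apply controller yaw and pitch directly.
; It binds to the custom EventCharMovementComponent's movement-mode-changed event, with debug prints for mode changes and node lookup.
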(event EventBeginPlay
  (Init|SetupInput)
  (Init|InitStateRefs)
  (bind _asevent_char_movement_component (Utilities|Casting|CastToEventCharMovementComponent (Variables|Character|GetCharacterMovement)))
  (EventDispatchers|BindEventtoMovementModeChangedEvent _asevent_char_movement_component (EventDispatchers|CreateEvent :!event BPStateMachineCharAutoGenFunc)))

(event Input|EnhancedActionEvents|EnhancedInputActionIA_Move
  (params (ActionValue :type Vector%202D%20Structure) (ElapsedSeconds :type Float%20%28double-precision%29) (TriggeredSeconds :type Float%20%28double-precision%29) (InputAction :type Input%20Action%20Object%20Reference :default "/Game/Assets/Input/IA_Move.IA_Move"))
  (:Triggered
    (Control|Movement|MovementContinue ActionValue))
  (:Started
    (Control|Movement|MovementStart))
  (:Canceled
    (Control|Movement|MovementStopped :!label _label))
  (:Completed
    (goto _label)))

(event Input|EnhancedActionEvents|EnhancedInputActionIA_Look
  (params (ActionValue :type Vector%202D%20Structure) (ElapsedSeconds :type Float%20%28double-precision%29) (TriggeredSeconds :type Float%20%28double-precision%29) (InputAction :type Input%20Action%20Object%20Reference :default "/Game/Assets/Input/IA_Look.IA_Look"))
  (:Triggered
    (Control|Camera|Look ActionValue)))

(fn ConstructionScript)

(fn InitStateRefs
  (bind _returnvalue (Class|ProcStateMachineComponent|FindNode (Variables|Default|GetProcStateMachine) "WALKING")
    (:FOUND
      (bind _asmovement_state_node (Utilities|Casting|CastToMovementStateNode _returnvalue)
        (:then
          (bind _output_get (Variables|StateMachine|States|SetWalkingStateNode _asmovement_state_node))
          (Development|PrintString (Utilities|String|Append (Utilities|GetDisplayName _output_get) "-- Found?")))
        (:CastFailed
          (Development|PrintString (Utilities|GetDisplayName _asmovement_state_node)))))
    (:NOTFOUND
      (Development|PrintString "Failed to find the node?"))))

(fn SetupInput
  (bind _asplayer_controller (Utilities|Casting|CastToPlayerController (Pawn|GetController)))
  (Input|AddMappingContext (PlayerController|LocalPlayerSubsystems|GetEnhancedInputLocalPlayerSubsystem _asplayer_controller) "/Game/Assets/Input/IMC_Default.IMC_Default" 0 "(bIgnoreAllPressedKeysUntilRelease=True,bForceImmediately=False)"))

(fn MovementStart
  (Class|ProcStateMachineComponent|Event (Variables|Default|GetProcStateMachine) (Variables|StateMachine|Events|Constants|GetWalkEventName)))

(fn MovementContinue
  (params (InputAxis :type Vector%202D%20Structure))
  (Class|MovementStateNode|UpdateInputAxis (Variables|StateMachine|States|GetWalkingStateNode) InputAxis))

(fn MovementStopped
  (Class|ProcStateMachineComponent|Event (Variables|Default|GetProcStateMachine) (Variables|StateMachine|Events|Constants|GetStopWalkEventName)))

(fn Look
  (params (LookAxis :type Vector%202D%20Structure))
  (Pawn|Input|AddControllerYawInput (.x LookAxis))
  (Pawn|Input|AddControllerPitchInput (.y LookAxis)))

(fn BPStateMachineCharAutoGenFunc
  (params (Component :type %20Object%20Reference) (Previous :type EMovementMode%20Enum :default "MOVE_None") (PreviousCustom :type Byte))
  (Development|PrintString (Utilities|String|EnumtoString Previous)))
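; Player character Blueprint that handles interaction, spell casting, target lock-on, damage, and pausing.
; It builds its inventory and caches a child-actor lock-on camera at construction, then initializes the main UI on BeginPlay.
; Interactables register themselves for popups and input-triggered use.
; Casting spawns the current spell and forwards notifies to it via BPI_Spell, while lock-on blends the view target and switches perspective and movement orientation.
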(event Custom|StartCast_1
  (if (not (Utilities|IsValid (Utilities|ToObject(Interface) (Variables|RPGElements|Casting|GetCastingSpell))))
    (SpellCasting|ChannelSpell)))

(event Input|EnhancedActionEvents|EnhancedInputActionIA_Interact
  (params (ActionValue :type Boolean) (ElapsedSeconds :type Float%20%28double-precision%29) (TriggeredSeconds :type Float%20%28double-precision%29) (InputAction :type Input%20Action%20Object%20Reference :default "/Game/Assets/Input/IA_Interact.IA_Interact"))
  (:Started
    (if (> (Utilities|Array|Length (Variables|Default|GetInteractObject)) 0)
      (Default|Interact (Utilities|Array|Get(acopy) (Variables|Default|GetInteractObject)) self))))

(event Input|EnhancedActionEvents|EnhancedInputActionIA_LockOn
  (params (ActionValue :type Boolean) (ElapsedSeconds :type Float%20%28double-precision%29) (TriggeredSeconds :type Float%20%28double-precision%29) (InputAction :type Input%20Action%20Object%20Reference :default "/Game/Assets/Input/IA_LockOn.IA_LockOn"))
  (:Started
    (if (Default|IsLockedon (Variables|Components|GetLockOnCameraRef))
      (LockOn|LockOff)
      (else
        (LockOn|Lockon)))))

(event Input|EnhancedActionEvents|EnhancedInputActionIA_OpenPause
  (params (ActionValue :type Boolean) (ElapsedSeconds :type Float%20%28double-precision%29) (TriggeredSeconds :type Float%20%28double-precision%29) (InputAction :type Input%20Action%20Object%20Reference :default "/Game/Assets/Input/IA_OpenPause.IA_OpenPause"))
  (:Started
    (CallFunction|Pause)))

(event EventBeginPlay
  (Initialization|InitInterface))

(event EventNotifyLaunch
  (Default|NotifyLaunch (Variables|RPGElements|Casting|GetCastingSpell) (Variables|/Game/Assets/Actors/Cameras/LockOnCamera/BP_LockOnCamera.BP_LockOnCamera_C|GetLockOnTarget (Variables|Components|GetLockOnCameraRef))))

(event EventNotifyChannel
  (Default|NotifyChannel (Variables|RPGElements|Casting|GetCastingSpell)))

(event EventDisplayPopup
  (params (Display%20Object :type BPI%20Displayable%20Interface))
  (Default|DisplayDialogue (Variables|Interface|GetMainUIRef) Display%20Object))

(event EventHidePopup
  (params (Display%20Object :type BPI%20Displayable%20Interface))
  (Default|HideDialogue (Variables|Interface|GetMainUIRef) Display%20Object))

(event EventDeclareInteractable
  (params (Interactable :type BPI%20Activator%20Interface))
  (bind _asbpi_displayable (Utilities|Casting|CastToBPI_Displayable Interactable))
  (Utilities|Array|Add (Variables|Default|GetInteractObject) Interactable)
  (Default|DisplayDialogue (Variables|Interface|GetMainUIRef) _asbpi_displayable))

(event EventRemoveInteractable
  (params (Interactor :type BPI%20Activator%20Interface))
  (Utilities|Array|RemoveItem (Variables|Default|GetInteractObject) Interactor)
  (bind _asbpi_displayable (Utilities|Casting|CastToBPI_Displayable Interactor))
  (CallFunction|HidePopup _asbpi_displayable))

(event EventTakeDamage
  (params (Hit%20Instance :type BP%20Hit%20Operator%20Object%20Reference))
  (Class|IntVariable|OperateValue (Variables|RPGElements|GetHealth) Hit%20Instance))

(event EventAttachSpell
  (params (Attach%20location :type BPE_SpellAttachLocation%20Enum :default "NewEnumerator0") (Socket%20Name :type Name :default "None") (Spell :type Actor%20Object%20Reference))
  (switch Utilities|FlowControl|Switch|SwitchonBPE_SpellAttachLocation Attach%20location
    (:NewEnumerator0
      (Transformation|AttachComponentToComponent Spell (Variables|Character|GetMesh) "hand_rSocket" "KeepRelative" "KeepRelative" "KeepRelative" true))))

(fn ConstructionScript
  (Utilities|FlowControl|Sequence
    (:then_0
      ;[1 1 1] Setup Inventory
      (bind _returnvalue (Game|ConstructObjectfromClass "/Game/Assets/RPGElements/Inventory/BP_Inventory.BP_Inventory_C"))
      (bind _output_get (Variables|RPGElements|Inventory|SetInventory _returnvalue))
      (Default|Initialize _output_get))
    (:then_1
      ;[1 1 1] Initialize Lockon Camera
      (bind _asbp_lock_on_camera (Utilities|Casting|CastToBP_LockOnCamera (Variables|/Script/Engine.ChildActorComponent|GetChildActor (Variables|Default|GetLock%20On%20Camera))))
      (Variables|Components|SetLockOnCameraRef _asbp_lock_on_camera))))

(fn InitInterface
  (bind _main_ui (Variables|Default|GetMain%20UI))
  (bind _returnvalue (UserInterface|GetWidget _main_ui))
  (UserInterface|Viewport|AddtoViewport _returnvalue 0)
  (bind _aswbp_main_ui (Utilities|Casting|CastToWBP_MainUI _returnvalue))
  (Variables|Interface|SetMainUIRef _aswbp_main_ui)
  (Default|Initialize _aswbp_main_ui self))

(fn Lockon
  (bind _lock_on_target_ (Default|Lockon (Variables|Components|GetLockOnCameraRef)))
  (if (Utilities|IsValid _lock_on_target_)
    (bind _asplayer_controller (Utilities|Casting|CastToPlayerController (Pawn|GetController)))
    (Game|Player|SetViewTargetwithBlend _asplayer_controller (Variables|Components|GetLockOnCameraRef) 0.5 "VTBlend_Linear" 0.0 false)
    (Class|PerspectiveManager|SetPerspective (Variables|Default|GetPerspectiveManager) (Variables|Components|GetLockOnCameraRef))
    (Variables|/Script/Engine.CharacterMovementComponent|SetbOrientRotationToMovement (Variables|Character|GetCharacterMovement self) false)
    (Variables|/Script/Engine.CameraComponent|SetbUsePawnControlRotation (Variables|Default|GetFollowCamera) false)))

(fn LockOff
  (bind _asplayer_controller (Utilities|Casting|CastToPlayerController (Pawn|GetController)))
  (Game|Player|SetViewTargetwithBlend _asplayer_controller self 0.5 "VTBlend_Linear" 0.0 false)
  (Class|PerspectiveManager|ResetPerspective (Variables|Default|GetPerspectiveManager))
  (Variables|/Script/Engine.CharacterMovementComponent|SetbOrientRotationToMovement (Variables|Character|GetCharacterMovement self) true)
  (Default|LockOff (Variables|Components|GetLockOnCameraRef)))

(fn ChannelSpell
  (bind (_returnvalue _spell_reference) (|CheckForCurrentSpell))
  (if _returnvalue
    (bind _asabp_playground_character (Utilities|Casting|CastToABP_PlaygroundCharacter (Components|SkeletalMesh|GetAnimInstance (Variables|Character|GetMesh))))
    (Default|SetCurrentSpell _asabp_playground_character _spell_reference)
    (bind _returnvalue_2 (Game|SpawnActorfromClass (Variables|/Game/Assets/RPGElements/Inventory/Spells/BP_SpellReference.BP_SpellReference_C|GetSpell%20Class _spell_reference) (Math|Transform|MakeTransform "0, 0, 0" "0, 0, 0" "1.000000,1.000000,1.000000") "Undefined" "MultiplyWithRoot" 0 0))
    (bind _asbpi_spell (Utilities|Casting|CastToBPI_Spell _returnvalue_2))
    (Default|Initialize _asbpi_spell self)
    (Variables|RPGElements|Casting|SetCastingSpell _asbpi_spell)))

(fn Pause
  (bind _returnvalue (Game|GetPlayerController 0))
  (bind _mainuiref (Variables|Interface|GetMainUIRef))
  (if (Variables|Default|GetIsPaused)
    (Variables|/Script/Engine.PlayerController|SetbShowMouseCursor _returnvalue false)
    (Variables|Default|SetIsPaused false)
    (Input|SetInputModeGameOnly _returnvalue false)
    (Class|GameplayStatics|SetViewportMouseCaptureMode "CapturePermanently")
    (Default|ClosePause _mainuiref)
    (else
      (Variables|/Script/Engine.PlayerController|SetbShowMouseCursor _returnvalue true)
      (Input|SetInputModeGameandUI _returnvalue (Variables|Interface|GetMainUIRef) "DoNotLock" true false)
      (Variables|Default|SetIsPaused true)
      (Default|OpenPause _mainuiref))))

(fn DeflectionCall)

(fn GetActor
  (return self))

(fn GetFactions
  (return (Variables|RPGElements|GetFactions)))

(fn GetHealth
  (return (Variables|RPGElements|GetHealth)))

(fn GetInventory
  (return 0))

(fn GetResponse
  (params (Other%20Entity :type Array%20of%20BP_Factions%20Enums :default "NewEnumerator0"))
  (return "NewEnumerator0"))
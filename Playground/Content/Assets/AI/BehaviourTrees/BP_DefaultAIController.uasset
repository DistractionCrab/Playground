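; AI controller for BP_BaseNPC pawns that runs the default behavior tree and feeds it perception results.
; On possession it starts BT_DefaultAI and copies the NPC's patrol path into PatrolRoute.
; Successfully sensed actors implementing BPI_RPGCharacter are written to the ObservedEntity blackboard key.
; Unsuccessful perception updates clear that key regardless of target, with debug prints throughout.
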(event OnTargetPerceptionUpdated(AIPerception)
  (params (Actor :type Actor%20Object%20Reference) (Stimulus :type AI%20Stimulus%20Structure))
  (if (Utilities|Struct|BreakAIStimulus Stimulus)
    (Development|PrintString (|printjunk Actor))
    (bind _asbpi_rpgcharacter (Utilities|Casting|CastToBPI_RPGCharacter Actor)
      (:then
        (AI|Components|Blackboard|SetValueasObject (Variables|Default|GetBlackboard) (Variables|Default|GetObserved%20Entity) (Utilities|ToObject(Interface) _asbpi_rpgcharacter)))
      (:CastFailed
        (Development|PrintString "Found Non RPG Character :(")))))

(event OnTargetPerceptionInfoUpdated(AIPerception)
  (params (UpdateInfo :type Actor%20Perception%20Update%20Info%20Structure%20%28by%20ref%29))
  (bind (_targetid _target _stimulus) (Utilities|Struct|BreakActorPerceptionUpdateInfo UpdateInfo))
  (bind _bsuccessfullysensed (Utilities|Struct|BreakAIStimulus _stimulus))
  (if (not _bsuccessfullysensed)
    (Development|PrintString (Utilities|String|Append (select _bsuccessfullysensed "Not Lost:" "Lost") (Utilities|GetDisplayName _target)))
    (AI|Components|Blackboard|SetValueasObject (Variables|Default|GetBlackboard) (Variables|Default|GetObserved%20Entity) 0)))

(event EventBeginPlay)

(event EventTick
  (params (DeltaSeconds :type Float%20%28single-precision%29)))

(event EventPossess
  (params (PossessedPawn :type Pawn%20Object%20Reference))
  (bind _asbp_base_npc (Utilities|Casting|CastToBP_BaseNPC PossessedPawn))
  (bind _output_get (Variables|Default|SetOwnerCasted _asbp_base_npc))
  (Development|PrintString "Possessed")
  (AI|RunBehaviorTree "/Game/Assets/AI/BehaviourTrees/BT_DefaultAI.BT_DefaultAI")
  (Variables|Default|SetPatrol%20Route (Variables|/Game/Assets/Actors/Entity/BP_BaseNPC.BP_BaseNPC_C|GetPatrol%20Path _output_get)))

(fn ConstructionScript)
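; BP_SpellBook is an RPG spell book that tracks owned and equipped spells.
; GetCurrentSpell returns the equipped spell at UseIndex when the equipped list is not empty.
; CycleSpells increments UseIndex without wrapping or clamping it, then returns the current spell.
; AddLearnedSpell adds a spell key to the owned spells, leaving the equipped list untouched.
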(fn GetCurrentSpell
  (bind _equipped_spells (Variables|Default|GetEquipped%20Spells))
  (return (select (> (Utilities|Array|Length _equipped_spells) 0) (Utilities|Array|Get(acopy) _equipped_spells (Variables|Default|GetUse%20Index)) 0)))

(fn CycleSpells
  (Math|Integer|IncrementInt (Variables|Default|GetUse%20Index)
    (:%20%20
      (bind _equipped_spell (CallFunction|GetCurrentSpell))
      (return _equipped_spell))))

(fn AddLearnedSpell
  (params (Spell%20Key :type String))
  (Utilities|Array|Add (Variables|Default|GetOwned%20Spells) Spell%20Key))
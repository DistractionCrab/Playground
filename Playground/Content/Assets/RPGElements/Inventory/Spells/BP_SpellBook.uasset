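; BP_SpellBook tracks the spells a character has learned and equipped, and which one is current.
; Learning adds a key to OwnedSpells after validating it against the SpellData table, then fires NewSpell.
; Equipping an owned key constructs a BP_SpellReference from its table row and appends it to EquippedSpells.
; Cycling increments UseIndex without wrapping, fires ChangeSpell from OwnedSpells, and returns the EquippedSpells entry at UseIndex.
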(fn GetCurrentSpell
  (bind _equipped_spells (Variables|Default|GetEquipped%20Spells))
  (return (select (> (Utilities|Array|Length _equipped_spells) 0) (Utilities|Array|Get(acopy) _equipped_spells (Variables|Default|GetUse%20Index)) 0)))

(fn CycleSpells
  (bind _result (Math|Integer|IncrementInt (Variables|Default|GetUse%20Index))
    (:%20%20
      (Default|CallChangeSpell (Utilities|Array|Get(acopy) (Variables|Default|GetOwned%20Spells) _result))
      (return (CallFunction|GetCurrentSpell)))))

(fn AddLearnedSpell
  (params (Spell%20Key :type Name))
  (bind _returnvalue (Class|DataTableFunctionLibrary|DoesDataTableRowExist (Variables|Default|GetSpell%20Data) Spell%20Key))
  (if _returnvalue
    (Utilities|Array|Add (Variables|Default|GetOwned%20Spells) Spell%20Key)
    (Default|CallNewSpell Spell%20Key)))

(fn EquipSpell
  (params (SpellKey :type Name))
  (if (Utilities|Array|ContainsItem (Variables|Default|GetOwned%20Spells) SpellKey)
    (bind _returnvalue (Utilities|GetDataTableRow (Variables|Default|GetSpell%20Data) SpellKey)
      (:then
        (bind _returnvalue_2 (Game|ConstructObjectfromClass "/Game/Assets/RPGElements/Inventory/Spells/BP_SpellReference.BP_SpellReference_C" _returnvalue (.SpellClass (Utilities|Struct|BreakSpellData _returnvalue))))
        (Utilities|Array|Add (Variables|Default|GetEquipped%20Spells) _returnvalue_2)))))